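; BP_Door is a double sliding door that opens once, with no logic to close it.
; BeginPlay caches each mesh's closed relative location and derives open locations offset in opposite directions along X.
; OpenDoor, guarded by the IsOpen flag, plays a sound at the actor and starts a timeline that lerps both panels apart.
; Nothing in this Blueprint calls OpenDoor itself.
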(event `OpenDoor`
  (if (not (`self.bIsOpen`))
    (set `self.bIsOpen` true)
    (`GameplayStatics.PlaySoundAtLocation` "/Game/Audio/Door.Door" (`self.K2_GetActorLocation`) (struct) 1.0 1.0 0.0 null null null null)
    (bind (_direction _alpha) (`Timeline|TL_OpenDoor` :!via `PlayFromStart`)
      (:`Update`
        (`SceneComponent.K2_SetRelativeLocation` (`self.LeftDoorMesh`) (`KismetMathLibrary.VLerp` (`self.LeftClosedLocation`) (`self.LeftOpenLocation`) _alpha) false false)
        (`SceneComponent.K2_SetRelativeLocation` (`self.RightDoor Mesh`) (`KismetMathLibrary.VLerp` (`self.RightClosedLocation`) (`self.RightOpenLocation`) _alpha) false false)))))

(event `self.ReceiveBeginPlay`
  (set `self.LeftClosedLocation` (`SceneComponent.RelativeLocation` (`self.LeftDoorMesh`)))
  (set `self.RightClosedLocation` (`SceneComponent.RelativeLocation` (`self.RightDoor Mesh`)))
  (set `self.LeftOpenLocation` (+ (`self.LeftClosedLocation`) (-120.0 0.0 0.0)))
  (set `self.RightOpenLocation` (+ (`self.RightClosedLocation`) (120.0 0.0 0.0))))

(fn `UserConstructionScript`)