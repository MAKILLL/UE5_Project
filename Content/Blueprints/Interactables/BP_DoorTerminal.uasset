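; BP_DoorTerminal is an interactable terminal that opens its linked door, optionally gated behind the player's door access.
; On Interact, a restricted terminal checks HasDoorAccess on the player character, then either opens the door or shows a Russian denial message, each with a sound.
; Unrestricted terminals open the door directly with the same feedback.
; The first authorized opening also updates the HUD objective to finding the control center, guarded by a one-time flag.
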(event `self.Interact`
  (if (`self.bRequiresAccess`)
    (bind _asfinal_project_character (cast `FinalProjectCharacter` (`GameplayStatics.GetPlayerCharacter` 0)))
    (if (`FinalProjectCharacter.bHasDoorAccess` _asfinal_project_character)
      (bind _asbp_first_person_character (cast `/Game/FirstPerson/Blueprints/BP_FirstPersonCharacter` (`GameplayStatics.GetPlayerCharacter` 0)))
      (`/Game/UI/WBP_HUD.ShowCenterMessage` (`/Game/FirstPerson/Blueprints/BP_FirstPersonCharacter.HUDWidget` _asbp_first_person_character) "Дверь открыта")
      (`GameplayStatics.PlaySound2D` "/Game/Audio/Access.Access" 1.0 1.0 0.0 null null)
      (`/Game/Blueprints/Doors/BP_Door.OpenDoor` (`self.LinkedDoor`))
      (if (not (`self.bObjectiveWasUpdated`))
        (bind _asbp_first_person_character_2 (cast `/Game/FirstPerson/Blueprints/BP_FirstPersonCharacter` (`GameplayStatics.GetPlayerCharacter` 0)))
        (`/Game/UI/WBP_HUD.SetObjectiveText` (`/Game/FirstPerson/Blueprints/BP_FirstPersonCharacter.HUDWidget` _asbp_first_person_character_2) "Цель: Найдите центр управления")
        (set `self.bObjectiveWasUpdated` true))
      (else
        (bind _asbp_first_person_character_3 (cast `/Game/FirstPerson/Blueprints/BP_FirstPersonCharacter` (`GameplayStatics.GetPlayerCharacter` 0)))
        (`/Game/UI/WBP_HUD.ShowCenterMessage` (`/Game/FirstPerson/Blueprints/BP_FirstPersonCharacter.HUDWidget` _asbp_first_person_character_3) "Отказано в доступе")
        (`GameplayStatics.PlaySound2D` "/Game/Audio/NoAccess.NoAccess" 1.0 1.0 0.0 null null)))
    (else
      (bind _asbp_first_person_character_4 (cast `/Game/FirstPerson/Blueprints/BP_FirstPersonCharacter` (`GameplayStatics.GetPlayerCharacter` 0)))
      (`/Game/UI/WBP_HUD.ShowCenterMessage` (`/Game/FirstPerson/Blueprints/BP_FirstPersonCharacter.HUDWidget` _asbp_first_person_character_4) "Дверь открыта")
      (`GameplayStatics.PlaySound2D` "/Game/Audio/Access.Access" 1.0 1.0 0.0 null null)
      (`/Game/Blueprints/Doors/BP_Door.OpenDoor` (`self.LinkedDoor`)))))

(fn `UserConstructionScript`)