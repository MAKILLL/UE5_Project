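; Interactable main computer that gates a terminal puzzle behind a keycard and grants ventilation terminal access.
; With a keycard, Interact opens WBP_TerminalPuzzle with a self reference, shows the cursor and disables character input.
; Without one, it shows a denial message, plays a sound and sets a find-keycard objective once.
; OnPuzzleCompleted announces access with a sound, then once updates the objective and sets HasVentilationAccess on the player.
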(event `/Game/Blueprints/Interfaces/BI_Interactable.Interact`
  (bind _returnvalue (`GameplayStatics.GetPlayerController` 0))
  (bind _asfinal_project_character (cast `FinalProjectCharacter` (`GameplayStatics.GetPlayerCharacter` 0)))
  (if (`FinalProjectCharacter.bHasKeycard` _asfinal_project_character)
    (bind _returnvalue_2 (`|CreateWidget` "/Game/UI/WBP_TerminalPuzzle.WBP_TerminalPuzzle_C" null self))
    (`UserWidget.AddToViewport` _returnvalue_2 0)
    (set `PlayerController.bShowMouseCursor` true _returnvalue)
    (`WidgetBlueprintLibrary.SetInputMode_GameAndUIEx` _returnvalue _returnvalue_2)
    (`self.DisableInput` (`GameplayStatics.GetPlayerCharacter` 0) (`GameplayStatics.GetPlayerController` 0))
    (else
      (bind _asbp_first_person_character (cast `/Game/FirstPerson/Blueprints/BP_FirstPersonCharacter` (`GameplayStatics.GetPlayerCharacter` 0)))
      (`/Game/UI/WBP_HUD.ShowCenterMessage` (`/Game/FirstPerson/Blueprints/BP_FirstPersonCharacter.HUDWidget` _asbp_first_person_character) "Отказано в доступе \nНужна ключ-карта")
      (`GameplayStatics.PlaySound2D` "/Game/Audio/NoAccess.NoAccess" 1.0 1.0 0.0 null null)
      (if (not (`self.bObjectiveWasUpdated`))
        (bind _asbp_first_person_character_2 (cast `/Game/FirstPerson/Blueprints/BP_FirstPersonCharacter` (`GameplayStatics.GetPlayerCharacter` 0)))
        (`/Game/UI/WBP_HUD.SetObjectiveText` (`/Game/FirstPerson/Blueprints/BP_FirstPersonCharacter.HUDWidget` _asbp_first_person_character_2) "Цель: Найдите ключ-карту в этой комнате")
        (set `self.bObjectiveWasUpdated` true)))))

(event `OnPuzzleCompleted`
  (bind _asbp_first_person_character (cast `/Game/FirstPerson/Blueprints/BP_FirstPersonCharacter` (`GameplayStatics.GetPlayerCharacter` 0)))
  (`/Game/UI/WBP_HUD.ShowCenterMessage` (`/Game/FirstPerson/Blueprints/BP_FirstPersonCharacter.HUDWidget` _asbp_first_person_character) "Получен доступ к терминалу вентиляции")
  (`GameplayStatics.PlaySound2D` "/Game/Audio/Access.Access" 1.0 1.0 0.0 null null)
  (if (not (`self.bObjectiveWasUpdated2`))
    (bind _asbp_first_person_character_2 (cast `/Game/FirstPerson/Blueprints/BP_FirstPersonCharacter` (`GameplayStatics.GetPlayerCharacter` 0)))
    (`/Game/UI/WBP_HUD.SetObjectiveText` (`/Game/FirstPerson/Blueprints/BP_FirstPersonCharacter.HUDWidget` _asbp_first_person_character_2) "Цель: Вернитесь к терминалу вентиляции")
    (bind _asfinal_project_character (cast `FinalProjectCharacter` (`GameplayStatics.GetPlayerCharacter` 0)))
    (set `FinalProjectCharacter.bHasVentilationAccess` true _asfinal_project_character)
    (set `self.bObjectiveWasUpdated2` true)))

(fn `UserConstructionScript`)