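; BP_Laptop2 is an interactable laptop that grants the player access to the control center door.
; Interact sets HasDoorAccess on the player character, shows a Russian unlock message through the HUD widget and plays an access sound.
; The ObjectiveWasUpdated flag limits the objective change to opening that door to one time, while the access grant, message and sound repeat on each successful use.
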(event `self.Interact`
  (bind _asfinal_project_character (cast `FinalProjectCharacter` (`GameplayStatics.GetPlayerCharacter` 0)))
  (set `FinalProjectCharacter.bHasDoorAccess` true _asfinal_project_character)
  (bind _asbp_first_person_character (cast `/Game/FirstPerson/Blueprints/BP_FirstPersonCharacter` (`GameplayStatics.GetPlayerCharacter` 0)))
  (`/Game/UI/WBP_HUD.ShowCenterMessage` (`/Game/FirstPerson/Blueprints/BP_FirstPersonCharacter.HUDWidget` _asbp_first_person_character) "Дверь к центру управления разблокирована")
  (`GameplayStatics.PlaySound2D` "/Game/Audio/Access.Access" 1.0 1.0 0.0 null null)
  (if (not (`self.bObjectiveWasUpdated`))
    (bind _asbp_first_person_character_2 (cast `/Game/FirstPerson/Blueprints/BP_FirstPersonCharacter` (`GameplayStatics.GetPlayerCharacter` 0)))
    (`/Game/UI/WBP_HUD.SetObjectiveText` (`/Game/FirstPerson/Blueprints/BP_FirstPersonCharacter.HUDWidget` _asbp_first_person_character_2) "Цель: Откройте дверь к центру управления")
    (set `self.bObjectiveWasUpdated` true)))

(fn `UserConstructionScript`)