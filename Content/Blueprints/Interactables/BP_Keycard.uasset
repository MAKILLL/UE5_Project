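; BP_Keycard is an interactable keycard pickup that grants the player the keycard and advances the objective.
; On Interact it sets HasKeycard on the FinalProjectCharacter, if not already set, then plays a 2D access sound.
; It casts the player to BP_FirstPersonCharacter to show a Russian pickup message and a new objective to find the control center on the HUD widget, then destroys itself.
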(event `/Game/Blueprints/Interfaces/BI_Interactable.Interact`
  (bind _asfinal_project_character (cast `FinalProjectCharacter` (`GameplayStatics.GetPlayerCharacter` 0)))
  (if (not (`FinalProjectCharacter.bHasKeycard` _asfinal_project_character))
    (set `FinalProjectCharacter.bHasKeycard` true _asfinal_project_character)
    (bind _asbp_first_person_character (cast `/Game/FirstPerson/Blueprints/BP_FirstPersonCharacter` (`GameplayStatics.GetPlayerCharacter` 0)))
    (`/Game/UI/WBP_HUD.ShowCenterMessage` (`/Game/FirstPerson/Blueprints/BP_FirstPersonCharacter.HUDWidget` _asbp_first_person_character) "Ключ-карта получена")
    (`GameplayStatics.PlaySound2D` "/Game/Audio/Access.Access" 1.0 1.0 0.0 null null)
    (bind _asbp_first_person_character_2 (cast `/Game/FirstPerson/Blueprints/BP_FirstPersonCharacter` (`GameplayStatics.GetPlayerCharacter` 0)))
    (`/Game/UI/WBP_HUD.SetObjectiveText` (`/Game/FirstPerson/Blueprints/BP_FirstPersonCharacter.HUDWidget` _asbp_first_person_character_2) "Цель: Найдите центр управления")
    (`self.K2_DestroyActor`)))

(fn `UserConstructionScript`)